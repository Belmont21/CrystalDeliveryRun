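; Quest component that tracks its owner's active quests and advances their objectives from gameplay events.
; AddQuest turns a quest definition into a runtime struct, skipping duplicate IDs, and announces the start.
; It binds to BP_QuestGameState's objective event, matching type and target ID against active quests' objectives.
; Matches add clamped progress, write the structs back into the array, then broadcast either completion or progress change.
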(event Custom|HandleGameplayObjective
  (params (ObjectiveType :type EQuestObjectiveType%20Enum :default "NewEnumerator0") (TargetID :type Name) (Amount :type Integer))
  (for (_array_element _array_index) (Variables|Default|GetActiveQuests)
    (if (and (.IsActive (Utilities|Struct|BreakST_QuestRuntime _array_element)) (not (.IsCompleted (Utilities|Struct|BreakST_QuestRuntime _array_element))))
      (for (_array_element_2 _array_index_2) (.Objectives (Utilities|Struct|BreakST_QuestRuntime _array_element))
        (if (and (Utilities|Enum|Equal(Enum) (.ObjectiveType (Utilities|Struct|BreakST_QuestObjective _array_element_2)) ObjectiveType) (== (.TargetID (Utilities|Struct|BreakST_QuestObjective _array_element_2)) TargetID))
          (CallFunction|UpdateObjectiveProgress _array_index _array_index_2 Amount))))))

(event EventBeginPlay
  (bind _asbp_quest_game_state (Utilities|Casting|CastToBP_QuestGameState (Game|GetGameState)))
  (EventDispatchers|BindEventtoOnGameplayObjectiveEvent _asbp_quest_game_state (delegate Custom|HandleGameplayObjective)))

(fn FindQuestbyID
  (params (QuestID :type Name))
  (bind (_array_element _array_index) (Utilities|Array|ForEachLoopwithBreak (Variables|Default|GetActiveQuests) :!label _label)
    (:LoopBody
      (if (== (.QuestID (Utilities|Struct|BreakST_QuestRuntime _array_element)) QuestID)
        (LocalVariables|SetFoundLocal true)
        (LocalVariables|SetQuestDataLocal _array_element)
        (LocalVariables|SetQuestIndexLocal _array_index)
        (goto _label Break)))
    (:Completed
      (return (LocalVariables|GetFoundLocal) (LocalVariables|GetQuestDataLocal) (LocalVariables|GetQuestIndexLocal)))))

(fn AddQuest
  (params (QuestDefinition :type PDA%20Quest%20Definition%20Object%20Reference))
  (bind _questid (Variables|/Game/Quests/Definitions/PDA_QuestDefinition.PDA_QuestDefinition_C|GetQuestID QuestDefinition))
  (bind _found (CallFunction|FindQuestbyID _questid))
  (if _found
    (return)
    (else
      (bind _structout (Utilities|Struct|SetmembersinST_QuestRuntime (LocalVariables|GetNewQuestRuntime) _questid QuestDefinition (Variables|/Game/Quests/Definitions/PDA_QuestDefinition.PDA_QuestDefinition_C|GetObjectives QuestDefinition) true false))
      (Utilities|Array|Add (Variables|Default|GetActiveQuests) _structout)
      (Default|CallOnQuestStarted _structout))))

(fn UpdateObjectiveProgress
  (params (QuestIndex :type Integer) (ObjectiveIndex :type Integer) (Amount :type Integer))
  (bind _activequests (Variables|Default|GetActiveQuests))
  (LocalVariables|SetQuestRuntimeLocal (Utilities|Array|Get(acopy) _activequests QuestIndex))
  (LocalVariables|SetObjectivesLocal (.Objectives (Utilities|Struct|BreakST_QuestRuntime (LocalVariables|GetQuestRuntimeLocal))))
  (LocalVariables|SetObjectiveLocal (Utilities|Array|Get(acopy) (LocalVariables|GetObjectivesLocal) ObjectiveIndex))
  (bind _structout (Utilities|Struct|SetmembersinST_QuestObjective (LocalVariables|GetObjectiveLocal) (Math|Integer|Min(Integer) (+ (.CurrentAmount (Utilities|Struct|BreakST_QuestObjective (LocalVariables|GetObjectiveLocal))) Amount) (.RequiredAmount (Utilities|Struct|BreakST_QuestObjective (LocalVariables|GetObjectiveLocal))))))
  (Utilities|Array|SetArrayElem (LocalVariables|GetObjectivesLocal) ObjectiveIndex _structout)
  (bind _structout_2 (Utilities|Struct|SetmembersinST_QuestRuntime (LocalVariables|GetQuestRuntimeLocal) (LocalVariables|GetObjectivesLocal)))
  (Utilities|Array|SetArrayElem _activequests QuestIndex _structout_2)
  (CallFunction|CheckQuestCompleted QuestIndex))

(fn CheckQuestCompleted
  (params (QuestIndex :type Integer))
  (bind _activequests (Variables|Default|GetActiveQuests))
  (LocalVariables|SetQuestRuntimeLocal (Utilities|Array|Get(acopy) _activequests QuestIndex))
  (bind _array_element (Utilities|Array|ForEachLoopwithBreak (.Objectives (Utilities|Struct|BreakST_QuestRuntime (LocalVariables|GetQuestRuntimeLocal))) :!label _label)
    (:LoopBody
      (if (not (>= (.CurrentAmount (Utilities|Struct|BreakST_QuestObjective _array_element)) (.RequiredAmount (Utilities|Struct|BreakST_QuestObjective _array_element))))
        (LocalVariables|SetAllObjectivesCompleted false)
        (goto _label Break)))
    (:Completed
      (if (LocalVariables|GetAllObjectivesCompleted)
        (bind _structout (Utilities|Struct|SetmembersinST_QuestRuntime (LocalVariables|GetQuestRuntimeLocal) false true))
        (Utilities|Array|SetArrayElem _activequests QuestIndex _structout)
        (Default|CallOnQuestCompleted _structout)
        (else
          (Default|CallOnQuestProgressChanged (LocalVariables|GetQuestRuntimeLocal)))))))