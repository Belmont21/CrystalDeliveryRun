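; Player character Blueprint for the C++ quest system, linking quest events to an on-screen tracker and handling interaction.
; On BeginPlay it creates the WBP_CPPQuestTracker widget and binds to its CDRQuestComponent's started, progress-changed and completed events, each refreshing the tracker with the quest data.
; IA_Interact sends an interact message, passing itself, to every overlapping actor implementing the CDRQuestInteractable interface.
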(event Custom|HandleCPPQuestStarted
  (params (QuestData :type CDR%20Quest%20Runtime%20Structure))
  (Default|UpdateQuestDisplay (Variables|Default|GetCPPQuestTracker) QuestData))

(event Custom|HandleCPPQuestProgress
  (params (QuestData :type CDR%20Quest%20Runtime%20Structure))
  (Default|UpdateQuestDisplay (Variables|Default|GetCPPQuestTracker) QuestData))

(event Custom|HandleCPPQuestCompleted
  (params (QuestData :type CDR%20Quest%20Runtime%20Structure))
  (Default|UpdateQuestDisplay (Variables|Default|GetCPPQuestTracker) QuestData))

(event Input|EnhancedActionEvents|EnhancedInputActionIA_Interact
  (params (ActionValue :type Boolean) (ElapsedSeconds :type Float%20%28double-precision%29) (TriggeredSeconds :type Float%20%28double-precision%29) (InputAction :type Input%20Action%20Object%20Reference :default "/Game/Input/Actions/IA_Interact.IA_Interact"))
  (:Started
    (for _array_element (Collision|GetOverlappingActors "/Script/Engine.Actor" :!class /Script/Engine.Actor)
      (if (Utilities|DoesObjectImplementInterface _array_element "/Script/CrystalDeliveryRun.CDRQuestInteractable")
        (Class|CDRQuestInteractable|Interact(Message) _array_element self)))))

(event EventBeginPlay
  (bind _returnvalue (Actor|GetComponentbyClass "/Script/CrystalDeliveryRun.CDRQuestComponent"))
  (bind _returnvalue_2 (UserInterface|CreateWidget "/Game/Quests/CPP/WBP_CPPQuestTracker.WBP_CPPQuestTracker_C" (Game|GetPlayerController 0)))
  (bind _output_get (Variables|Default|SetCPPQuestTracker _returnvalue_2))
  (UserInterface|Viewport|AddtoViewport _output_get 0)
  (EventDispatchers|BindEventtoOnQuestStarted _returnvalue (delegate Custom|HandleCPPQuestStarted))
  (EventDispatchers|BindEventtoOnQuestProgressChanged _returnvalue (delegate Custom|HandleCPPQuestProgress))
  (EventDispatchers|BindEventtoOnQuestCompleted _returnvalue (delegate Custom|HandleCPPQuestCompleted)))

(fn ConstructionScript
  (|CallParentFunction))